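; Play-level game mode that spawns the player's character and skin as stored in the game instance.
; On BeginPlay it reads the saved selection and spawns either the Countess or Sun Wukong character at the player start.
; After a short delay it applies the chosen skeletal mesh, if one is valid, then has the first player controller possess the character.
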(event `self.ReceiveBeginPlay`
  (bind (_skin_index _nhanvat _skin_chon) (message `/Game/Than/Menu_game/menu_nhanvat/Skin_nhanvat.lood_Skin` (`GameplayStatics.GetGameInstance`)))
  (bind _returnvalue (`|SpawnActorFromClass` (select `bool` _nhanvat :`false` "/Game/Than/SunWukongPlayerCharacter.SunWukongPlayerCharacter_C" :`true` "/Game/Than/AI_countess/CountessPlayerCharacter.CountessPlayerCharacter_C" :!type "Actor Class Reference") (`self.GetTransform` (`self.K2_FindPlayerStart` null)) "Undefined" "OverrideRootScale"))
  (`KismetSystemLibrary.Delay` 0.2)
  (bind _ascharacter (cast `Character` _returnvalue))
  (`/Engine/EditorBlueprintResources/StandardMacros.IsValid` _skin_chon
    (:`Is Valid`
      (`SkinnedMeshComponent.SetSkinnedAssetAndUpdate` (`Character.Mesh` _ascharacter) _skin_chon true))
    (:`Is Not Valid`
      _))
  (`Controller.Possess` (`GameplayStatics.GetPlayerController` 0) _ascharacter))

(fn `UserConstructionScript`)